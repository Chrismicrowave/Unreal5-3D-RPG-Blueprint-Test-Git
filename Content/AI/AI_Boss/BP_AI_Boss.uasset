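; BP_AI_Boss is the boss AI character Blueprint, which reports its health to its AI controller.
; Every Tick it casts its controller to BP_AI_Controller_Boss and copies MaxHealth and CurHealth from the BPCNpcStats component into it.
; The sync is polled each frame, and the construction script only calls the parent.
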(event `self.ReceiveTick`
  (params (DeltaSeconds :type "Float (single-precision)"))
  (bind _bpc_npcstats (`self.BPC_NpcStats`))
  (`parent.ReceiveTick` DeltaSeconds)
  (bind _asbp_ai_controller_generic_boss (cast `/Game/AI/AI_Boss/BP_AI_Controller_Boss` (`AIBlueprintHelperLibrary.GetAIController` self)))
  (set `/Game/AI/AI_Boss/BP_AI_Controller_Boss.MaxHealth` (`/Game/Blueprints/BPC_NpcStats.MaxHealth` _bpc_npcstats) _asbp_ai_controller_generic_boss)
  (set `/Game/AI/AI_Boss/BP_AI_Controller_Boss.CurHealth` (`/Game/Blueprints/BPC_NpcStats.CurHealth` _bpc_npcstats) _asbp_ai_controller_generic_boss))

(fn `UserConstructionScript`
  (`parent.UserConstructionScript`))
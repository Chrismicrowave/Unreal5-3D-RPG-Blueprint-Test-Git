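; AI controller for a boss that runs the BT_AI_Boss behavior tree on begin play and manages the boss health bar.
; Activate and deactivate combat events create and remove the WB_Boss_HealthBar widget in the viewport.
; Every tick, while that widget is valid, it pushes CurHealth and MaxHealth into the bar's percentage and text by polling rather than reacting to damage events.
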(event `self.ReceiveBeginPlay`
  (`self.RunBehaviorTree` "/Game/AI/AI_Boss/BT_AI_Boss.BT_AI_Boss"))

(event `self.ReceiveTick`
  (params (DeltaSeconds :type "Float (single-precision)"))
  (`self.HpBarUpdate`))

(event `ActivateBossCombat`
  (bind _returnvalue (`|CreateWidget` "/Game/UI/WB_Boss_HealthBar.WB_Boss_HealthBar_C"))
  (bind _output_get (set `self.BossHPWidget` _returnvalue))
  (`UserWidget.AddToViewport` _output_get 0))

(event `DeactivateBossCombat`
  (`Widget.RemoveFromParent` (`self.BossHPWidget`))
  (set `self.BossHPWidget` null))

(event `HpBarUpdate`
  (bind _curhealth (`self.CurHealth`))
  (bind _maxhealth (`self.MaxHealth`))
  (bind _bosshpwidget (`self.BossHPWidget`)
    (:`then`
      (`ProgressBar.SetPercent` (`/Game/UI/WB_Boss_HealthBar.HealthBar` _bosshpwidget) (/ _curhealth _maxhealth))
      (set `TextBlock.Text` (`|FormatText` "{CurHp} / {MaxHp}" _curhealth _maxhealth) (`/Game/UI/WB_Boss_HealthBar.HpTxt` _bosshpwidget)))
    (:`else`)))

(fn `UserConstructionScript`
  (`parent.UserConstructionScript`))
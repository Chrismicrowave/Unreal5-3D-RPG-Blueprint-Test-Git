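; Player stats component tracking health, stamina, XP and level for BP_ThirdPersonCharacter and mirroring them to its HUD widget.
; On BeginPlay it waits a tick, caches the owning character and fills the bars; each change function then refreshes its bar and text.
; Decrease functions return true on depletion, and increases clamp to max.
; XP overflow converts to levels via division with remainder, raising MaxXP by a flat step and playing a sound.
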(event `self.ReceiveBeginPlay`
  (`KismetSystemLibrary.DelayUntilNextTick`)
  (bind _asbp_third_person_character (cast `/Game/ThirdPerson/Blueprints/BP_ThirdPersonCharacter` (`self.GetOwner`)))
  (set `self.PlayerCharacterBP` _asbp_third_person_character)
  (`self.HpBarUpdate`)
  (`self.StaBarUpdate`)
  (`self.XpLvlBarUpdate`))

(fn `HealthDecrease`
  (params (Damage :type "Float (double-precision)"))
  (returns (IsPlayerDead :type Boolean))
  (if (> (`self.CurHealth`) 0.0)
    (set `self.CurHealth` (- (`self.CurHealth`) Damage))
    (`self.HpBarUpdate`)
    (if (<= (`self.CurHealth`) 0.0)
      _
      (else
        (return false))))
  (return true))

(fn `HealthIncrease`
  (params (HealthUp :type "Float (double-precision)"))
  (set `self.CurHealth` (+ (`self.CurHealth`) HealthUp))
  (if (> (`self.CurHealth`) (`self.MaxHealth`))
    (set `self.CurHealth` (`self.MaxHealth`)))
  (`self.HpBarUpdate`))

(fn `HpBarUpdate`
  (`ProgressBar.SetPercent` (`/Game/UI/WB_HUD.HealthBar` (`/Game/ThirdPerson/Blueprints/BP_ThirdPersonCharacter.HudWidget` (`self.PlayerCharacterBP`))) (/ (`self.CurHealth`) (`self.MaxHealth`)))
  (`TextBlock.SetText` (`/Game/UI/WB_HUD.HpTxt` (`/Game/ThirdPerson/Blueprints/BP_ThirdPersonCharacter.HudWidget` (`self.PlayerCharacterBP`))) (`|FormatText` "{CurHp} / {MaxHp}" (`self.CurHealth`) (`self.MaxHealth`))))

(fn `LevelUp`
  (params (LevelUpNum :type "Float (double-precision)") (XpCarriedOver :type "Float (double-precision)"))
  (set `self.Level` (+ (`self.Level`) LevelUpNum))
  (set `self.MaxXP` (+ (`self.MaxXP`) 150.0))
  (set `self.XP` (+ 0.0 XpCarriedOver))
  (`self.XpLvlBarUpdate`)
  (`GameplayStatics.PlaySound2D` "/Game/Audio/UI/whoosh-epic-level-up.whoosh-epic-level-up" 1.0 1.0 0.0 null null))

(fn `MaxHealthIncrease`
  (params (MaxHealthUp :type "Float (double-precision)"))
  (set `self.MaxHealth` (+ (`self.MaxHealth`) MaxHealthUp))
  (`self.HpBarUpdate`))

(fn `MaxStaminaIncrease`
  (params (MaxStaminaUp :type "Float (double-precision)"))
  (set `self.MaxStamina` (+ (`self.MaxStamina`) MaxStaminaUp))
  (`self.StaBarUpdate`))

(fn `StaBarUpdate`
  (`self.PlayerCharacterBP`
    (:`then`
      (`ProgressBar.SetPercent` (`/Game/UI/WB_HUD.StaminaBar` (`/Game/ThirdPerson/Blueprints/BP_ThirdPersonCharacter.HudWidget` (`self.PlayerCharacterBP`))) (/ (`self.CurStamina`) (`self.MaxStamina`)))
      (`TextBlock.SetText` (`/Game/UI/WB_HUD.StaTxt` (`/Game/ThirdPerson/Blueprints/BP_ThirdPersonCharacter.HudWidget` (`self.PlayerCharacterBP`))) (`|FormatText` "{CurSta} / {MaxSta}" (`self.CurStamina`) (`self.MaxStamina`))))
    (:`else`)))

(fn `StaminaDecrease`
  (params (StaminaDepleted :type "Float (double-precision)"))
  (returns (NoStamina :type Boolean))
  (if (> (`self.CurStamina`) 0.0)
    (set `self.CurStamina` (- (`self.CurStamina`) StaminaDepleted))
    (`self.StaBarUpdate`)
    (if (<= (`self.CurStamina`) 0.0)
      _
      (else
        (return false))))
  (return true))

(fn `StaminaIncrease`
  (params (StaminaUp :type "Float (double-precision)"))
  (set `self.CurStamina` (+ (`self.CurStamina`) StaminaUp))
  (if (> (`self.CurStamina`) (`self.MaxStamina`))
    (set `self.CurStamina` (`self.MaxStamina`)))
  (`self.StaBarUpdate`))

(fn `XpIncrease`
  (params (XpGain :type "Float (double-precision)"))
  (bind _xp (`self.XP`))
  (bind _maxxp (`self.MaxXP`))
  (bind (_remainder _returnvalue) (`KismetMathLibrary.FMod` _xp _maxxp))
  (set `self.XP` (+ (`self.XP`) XpGain))
  (`self.XpLvlBarUpdate`)
  (if (>= _xp _maxxp)
    (bind _output_get (set `self.XpOver` _remainder))
    (`self.LevelUp` (`KismetMathLibrary.Conv_IntToDouble` _returnvalue) _output_get)
    (`self.XpLvlBarUpdate`)))

(fn `XpLvlBarUpdate`
  (bind _xp (`self.XP`))
  (bind _maxxp (`self.MaxXP`))
  (bind _hudwidget (`/Game/ThirdPerson/Blueprints/BP_ThirdPersonCharacter.HudWidget` (`self.PlayerCharacterBP`)))
  (`ProgressBar.SetPercent` (`/Game/UI/WB_HUD.XpBar` _hudwidget) (/ _xp _maxxp))
  (`TextBlock.SetText` (`/Game/UI/WB_HUD.XpTxt` _hudwidget) (`|FormatText` "{curXp} / {maxXp}" _xp _maxxp))
  (`TextBlock.SetText` (`/Game/UI/WB_HUD.LvlTxt` _hudwidget) (`|FormatText` "{level}" (`self.Level`))))
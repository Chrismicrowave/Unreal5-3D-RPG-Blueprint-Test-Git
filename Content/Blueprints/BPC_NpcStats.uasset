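; BPC_NpcStats is an actor component that holds current and maximum health for an NPC and drives its health bar.
; On BeginPlay it waits a tick, caches its owner as BP_Dummy and refreshes the bar.
; Decrease, capped increase and max-health functions each update the widget's fill percent and text.
; HealthDecrease returns true when health is depleted, and the bar update only works on BP_Dummy owners.
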(event `self.ReceiveBeginPlay`
  (`KismetSystemLibrary.DelayUntilNextTick`)
  (bind _asbp_dummy (cast `/Game/Blueprints/BP_Dummy` (`self.GetOwner`)))
  (set `self.AsBPDummy` _asbp_dummy)
  (`self.HpBarUpdate`))

(fn `HealthDecrease`
  (params (Damage :type "Float (double-precision)"))
  (returns (IsNpcDead :type Boolean))
  (if (> (`self.CurHealth`) 0.0)
    (set `self.CurHealth` (- (`self.CurHealth`) Damage))
    (`self.HpBarUpdate`)
    (if (<= (`self.CurHealth`) 0.0)
      _
      (else
        (return false))))
  (return true))

(fn `HealthIncrease`
  (params (HealthUp :type "Float (double-precision)"))
  (set `self.CurHealth` (+ (`self.CurHealth`) HealthUp))
  (if (> (`self.CurHealth`) (`self.MaxHealth`))
    (set `self.CurHealth` (`self.MaxHealth`)))
  (`self.HpBarUpdate`))

(fn `HpBarUpdate`
  (bind _asbpdummy (`self.AsBPDummy`))
  (bind _npchealthbarwidget (`/Game/Blueprints/BP_Dummy.NpcHealthBarWidget` _asbpdummy))
  (`/Engine/EditorBlueprintResources/StandardMacros.IsValid` _asbpdummy
    (:`Is Valid`
      (`ProgressBar.SetPercent` (`/Game/UI/WB_NPC.HpBar` _npchealthbarwidget) (/ (`self.CurHealth`) (`self.MaxHealth`)))
      (set `TextBlock.Text` (`|FormatText` "{CurHp} / {MaxHp}" (`self.CurHealth`) (`self.MaxHealth`)) (`/Game/UI/WB_NPC.HpTxt` _npchealthbarwidget)))))

(fn `MaxHealthIncrease`
  (params (MaxHealthUp :type "Float (double-precision)"))
  (set `self.MaxHealth` (+ (`self.MaxHealth`) MaxHealthUp))
  (`self.HpBarUpdate`))
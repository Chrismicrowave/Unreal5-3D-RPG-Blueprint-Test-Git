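; BP_Dummy is an NPC target dummy that can be hit or stealth-assassinated from behind, with a health bar and an assassination prompt.
; Damage plays a random hit montage, launches it along the player's forward vector and updates BPCNpcStats, ragdolling it when HealthDecrease returns true.
; StealthBackAssassin plays a paired victim montage, schedules a delayed ragdoll and returns a reference location and rotation.
; The prompt appears on player overlap, and both widgets face the camera every tick.
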(event `self.ReceiveBeginPlay`
  ;[1 1 1] Create NpcHealthBarWidget Component
  (bind _aswb_npc (cast `/Game/UI/WB_NPC` (`WidgetComponent.GetWidget` (`self.NpcHealthBar`))))
  (set `self.NpcHealthBarWidget` _aswb_npc)
  (`/Game/Blueprints/BPC_NpcStats.HpBarUpdate` (`self.BPC_NpcStats`)))

(event `Ragdoll`
  ;[1 1 1] Ragdoll
  (`|ExecutionSequence`
    (:`then_0`
      (`KismetSystemLibrary.Delay` 2.5)
      (`PrimitiveComponent.SetSimulatePhysics` (`self.Mesh`) true))
    (:`then_1`
      (`KismetSystemLibrary.Delay` 1.8)
      (`GameplayStatics.PlaySoundAtLocation` "/Game/Audio/Grunts-Hits/SC_Death.SC_Death" (`self.K2_GetActorLocation`) (struct) 1.0 1.0 0.0 "/Game/Audio/SA_Character.SA_Character" null null null))))

(event `self.AssassinPrompt.OnComponentBeginOverlap`
  (params (OverlappedComponent :type "PrimitiveComponent Object Reference") (OtherActor :type "Actor Object Reference") (OtherComp :type "PrimitiveComponent Object Reference") (OtherBodyIndex :type Integer) (bFromSweep :type Boolean) (SweepResult :type "HitResult Structure (by ref)"))
  ;[1 1 1] Widget Prompt
  (cast `/Game/ThirdPerson/Blueprints/BP_ThirdPersonCharacter` OtherActor)
  (`SceneComponent.SetVisibility` (`self.AssassinPrompt`) true false))

(event `self.AssassinPrompt.OnComponentEndOverlap`
  (params (OverlappedComponent :type "PrimitiveComponent Object Reference") (OtherActor :type "Actor Object Reference") (OtherComp :type "PrimitiveComponent Object Reference") (OtherBodyIndex :type Integer))
  ;[1 1 1] Widget Prompt
  (cast `/Game/ThirdPerson/Blueprints/BP_ThirdPersonCharacter` OtherActor)
  (`SceneComponent.SetVisibility` (`self.AssassinPrompt`) false false))

(event `self.ReceiveTick`
  (params (DeltaSeconds :type "Float (single-precision)"))
  (`self.AssassinPromptRotation`))

(event `AssassinPromptRotation`
  ;[1 1 1] Widget Rotation
  (`SceneComponent.K2_SetWorldRotation` (`self.AssassinPrompt`) (`KismetMathLibrary.FindLookAtRotation` (`SceneComponent.K2_GetComponentLocation` (`self.AssassinPrompt`)) (`SceneComponent.K2_GetComponentLocation` (`PlayerCameraManager.TransformComponent` (`GameplayStatics.GetPlayerCameraManager` 0)))) false false)
  (`SceneComponent.K2_SetWorldRotation` (`self.NpcHealthBar`) (`KismetMathLibrary.FindLookAtRotation` (`SceneComponent.K2_GetComponentLocation` (`self.AssassinPrompt`)) (`SceneComponent.K2_GetComponentLocation` (`PlayerCameraManager.TransformComponent` (`GameplayStatics.GetPlayerCameraManager` 0)))) false false))

(event `self.ReceiveAnyDamage`
  (params (Damage :type "Float (single-precision)") (DamageType :type "DamageType Object Reference") (InstigatedBy :type "Controller Object Reference") (DamageCauser :type "Actor Object Reference"))
  ;[1 1 1] AnyDamage
  (`self.PlayAnimMontage` (`|GetArrayItem` (`self.HitReactAnim`) (`KismetMathLibrary.RandomIntegerInRange` 0 (- (`KismetArrayLibrary.Array_Length` (`self.HitReactAnim`)) 1))))
  (bind _asbp_third_person_character (cast `/Game/ThirdPerson/Blueprints/BP_ThirdPersonCharacter` (`GameplayStatics.GetPlayerCharacter` 0)))
  (`self.LaunchCharacter` (* (`KismetMathLibrary.GetForwardVector` (`self.K2_GetActorRotation` _asbp_third_person_character)) 700.0))
  (`GameplayStatics.PlaySoundAtLocation` "/Game/Audio/Grunts-Hits/Death-Grunt2.Death-Grunt2" (`self.K2_GetActorLocation`) (struct) 1.0 (`KismetMathLibrary.RandomFloatInRange` 1.0 1.5) 0.0 "/Game/Audio/SA_Character.SA_Character" null null null)
  (bind _isnpcdead (`/Game/Blueprints/BPC_NpcStats.HealthDecrease` (`self.BPC_NpcStats`) Damage))
  (if _isnpcdead
    (`PrimitiveComponent.SetSimulatePhysics` (`self.Mesh`) true)
    (`GameplayStatics.PlaySoundAtLocation` "/Game/Audio/Grunts-Hits/SC_Death.SC_Death" (`self.K2_GetActorLocation`) (struct) 1.0 1.0 0.0 "/Game/Audio/SA_Character.SA_Character" null null null)
    (`SceneComponent.SetVisibility` (`self.NpcHealthBar`) false false)))

(fn `StealthBackAssassin`
  (returns (RefLocation :type "Vector Structure") (Rotation :type "Rotator Structure"))
  (`self.PlayAnimMontage` "/Game/Characters/RPG_Character/Animation/Assassination/Paired_Knife_Stealth_KidneyAndNeck_Vic_Montage.Paired_Knife_Stealth_KidneyAndNeck_Vic_Montage")
  (`self.Ragdoll`)
  (`SceneComponent.SetVisibility` (`self.AssassinPrompt`) false false)
  (return (`SceneComponent.K2_GetComponentLocation` (`self.AssassinRef`)) (`self.K2_GetActorRotation`)))

(fn `UserConstructionScript`)
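; Melee attack component for BP_ThirdPersonCharacter that runs a four-step sword and kick combo from IA_Attack input.
; Presses during an attack buffer the next step, which CombContinute either plays as a montage or ends by resetting the combo.
; Montage notify states start a timer-looped sphere trace along the blade, while HitSphereTrace makes a one-shot check.
; Hits on "Damageable" actors apply damage, camera shake, sound and blood, briefly throttled for blade traces.
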(event `self.ReceiveBeginPlay`
  (bind _asbp_third_person_character (cast `/Game/ThirdPerson/Blueprints/BP_ThirdPersonCharacter` (`self.GetOwner`)))
  (set `self.CharacterBP` _asbp_third_person_character)
  (set `self.ChracterMesh` (`Character.Mesh` _asbp_third_person_character)))

(event `EnhancedInput|/Game/ThirdPerson/Input/Actions/IA_Attack`
  (params (ActionValue :type Boolean) (ElapsedSeconds :type "Float (double-precision)") (TriggeredSeconds :type "Float (double-precision)") (InputAction :type "InputAction Object Reference" :default "/Game/ThirdPerson/Input/Actions/IA_Attack.IA_Attack"))
  (:`Started`
    (if (`self.CanAttack`)
      (`self.SwordAttack`))))

(event `SwordAttackCombo1`
  ;[1 1 1] Combo system
  ;;[1 1 1] SwordAttack1
  (`/Engine/EditorBlueprintResources/StandardMacros.DoOnce` false :!label _label
    (:`Completed`
      (`KismetSystemLibrary.Delay` 0.1)
      (`|PlayMontage` (`self.ChracterMesh`) "/Game/Characters/RPG_Character/Animation/SwordAttack/Attack1_Montage.Attack1_Montage"
        (:`then`
          (set `self.AttackIndex` 1)
          (goto _label :!via `Reset`))))))

(event `SwordAttack`
  ;[1 1 1] Combo system
  ;;[1 1 1] Sword Attack
  (if (`self.IsAttacking`)
    (set `self.NextCombo` true)
    (else
      (set `self.IsAttacking` true)
      (switch `int` (`self.AttackIndex`) :!label _label_2
        (:`0`
          (`self.SwordAttackCombo1`))
        (:`1`
          (`self.SwordAttackCombo2`))
        (:`2`
          (`self.SwordAttackCombo3`))
        (:`3`
          (`self.SwordAttackCombo4`))))))

(event `CombContinute`
  ;[1 1 1] Combo system
  ;;[1 1 1] Combo Continue
  (if (`self.NextCombo`)
    (set `self.NextCombo` false)
    (goto _label_2)
    (else
      (`self.StopCombo`))))

(event `SwordAttackCombo2`
  ;[1 1 1] Combo system
  ;;[1 1 1] SwordAttack2
  (`/Engine/EditorBlueprintResources/StandardMacros.DoOnce` false :!label _label_3
    (:`Completed`
      (`KismetSystemLibrary.Delay` 0.1)
      (`|PlayMontage` (`self.ChracterMesh`) "/Game/Characters/RPG_Character/Animation/SwordAttack/Attack2_Montage.Attack2_Montage"
        (:`then`
          (set `self.AttackIndex` 2)
          (goto _label_3 :!via `Reset`))))))

(event `StopCombo`
  ;[1 1 1] Combo system
  ;;[1 1 1] Stop Combo/Attack
  (set `self.IsAttacking` false)
  (set `self.AttackIndex` 0))

(event `SwordAttackCombo3`
  ;[1 1 1] Combo system
  ;;[1 1 1] SwordAttack3
  (`/Engine/EditorBlueprintResources/StandardMacros.DoOnce` false :!label _label_4
    (:`Completed`
      (`KismetSystemLibrary.Delay` 0.1)
      (`|PlayMontage` (`self.ChracterMesh`) "/Game/Characters/RPG_Character/Animation/SwordAttack/Kick_Montage.Kick_Montage"
        (:`then`
          (set `self.AttackIndex` 3)
          (goto _label_4 :!via `Reset`))))))

(event `SwordAttackCombo4`
  ;[1 1 1] Combo system
  ;;[1 1 1] SwordAttack4
  (`/Engine/EditorBlueprintResources/StandardMacros.DoOnce` false :!label _label_5
    (:`Completed`
      (`KismetSystemLibrary.Delay` 0.1)
      (`|PlayMontage` (`self.ChracterMesh`) "/Game/Characters/RPG_Character/Animation/SwordAttack/Attack3_Montage.Attack3_Montage"
        (:`then`
          (set `self.AttackIndex` 4)
          (goto _label_5 :!via `Reset`))))))

(event `StartSwordTrace`
  ;[1 1 1] SwordTrace Called in Montage AnimNotifyState
  (bind _returnvalue (`KismetSystemLibrary.K2_SetTimerDelegate` (delegate `SwordTraceLoop`) 0.01 true))
  (set `self.SwordTraceLoopHandle` _returnvalue))

(event `SwordTraceLoop`
  (bind _characterbp (`self.CharacterBP`))
  ;[1 1 1] SwordTrace Called in Montage AnimNotifyState
  (bind (_outhit _returnvalue) (`KismetSystemLibrary.SphereTraceSingle` :`Start` (`SceneComponent.K2_GetComponentLocation` (`/Game/ThirdPerson/Blueprints/BP_ThirdPersonCharacter.SwordTip` _characterbp)) :`End` (`SceneComponent.K2_GetComponentLocation` (`/Game/ThirdPerson/Blueprints/BP_ThirdPersonCharacter.SwordBottom` _characterbp)) :`Radius` 12.0 :`TraceChannel` "TraceTypeQuery1" :`DrawDebugType` "ForDuration" :`DrawTime` 0.1))
  (if _returnvalue
    (bind (_bblockinghit _binitialoverlap _time _distance _location _impactpoint _normal _impactnormal _physmat _hitactor) (`GameplayStatics.BreakHitResult` _outhit))
    (if (`Actor.ActorHasTag` _hitactor "Damageable")
      (`/Engine/EditorBlueprintResources/StandardMacros.DoOnce` false :!label _label_6
        (:`Completed`
          (`GameplayStatics.ApplyDamage` _hitactor 25.0)
          (`GameplayStatics.PlayWorldCameraShake` "/Game/Blueprints/BP_SwordHitCameraShake.BP_SwordHitCameraShake_C" _location 0.0 2000.0)
          (`self.PlaySwordHitSound`)
          (`GameplayStatics.SpawnEmitterAtLocation` "/Game/FX/SimpleBlood/Particles/Blood/P_SimpleBlood_Splat_Cone.P_SimpleBlood_Splat_Cone" _location (`KismetMathLibrary.MakeRotFromXY` _normal _normal) (0.4 0.4 0.4) true "AutoRelease")
          (`KismetSystemLibrary.Delay` 0.1)
          (goto _label_6 :!via `Reset`))))))

(event `StopSwordTrace`
  ;[1 1 1] SwordTrace Called in Montage AnimNotifyState
  (`KismetSystemLibrary.K2_ClearAndInvalidateTimerHandle` (`self.SwordTraceLoopHandle`)))

(event `HitSphereTrace`
  (bind _returnvalue (`SceneComponent.K2_GetComponentLocation` (`/Game/ThirdPerson/Blueprints/BP_ThirdPersonCharacter.HitSphereTrace` (`self.CharacterBP`))))
  ;[1 1 1] HitSphereTrace
  (bind (_outhit _returnvalue_2) (`KismetSystemLibrary.SphereTraceSingle` :`Start` _returnvalue :`End` _returnvalue :`Radius` 25.0 :`TraceChannel` "TraceTypeQuery1" :`DrawDebugType` "ForDuration"))
  (if _returnvalue_2
    (bind (_bblockinghit _binitialoverlap _time _distance _location _impactpoint _normal _impactnormal _physmat _hitactor) (`GameplayStatics.BreakHitResult` _outhit))
    (if (`Actor.ActorHasTag` _hitactor "Damageable")
      (`GameplayStatics.ApplyDamage` _hitactor 25.0)
      (`GameplayStatics.PlayWorldCameraShake` "/Game/Blueprints/BP_SwordHitCameraShake.BP_SwordHitCameraShake_C" _location 0.0 2000.0)
      (`self.PlaySwordHitSound`)
      (`GameplayStatics.SpawnEmitterAtLocation` "/Game/FX/SimpleBlood/Particles/Blood/P_SimpleBlood_Splat_Cone.P_SimpleBlood_Splat_Cone" _location (`KismetMathLibrary.MakeRotFromXY` _normal _normal) (0.4 0.4 0.4) true "AutoRelease")
      (`KismetSystemLibrary.Delay` 0.1))))

(event `PlaySwordHitSound`
  ;[1 1 1] Play SwordHit Sound
  (`GameplayStatics.PlaySoundAtLocation` "/Game/Audio/SwordHit/MS_SwordHit.MS_SwordHit" (`Actor.K2_GetActorLocation` (`self.GetOwner`)) (struct) 1.0 1.0 0.0 null null null null))